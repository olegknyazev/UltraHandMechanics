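; BP_PlayerUIController manages the crosshair UI for its owning UHPlayerController, showing it only during Ultra Hand Picking.
; On BeginPlay it caches the controller and creates a crosshairs widget.
; Each Tick it polls the control mode and, on a change, adds the widget to the player screen for picking or removes it for Regular, Manipulation and Turning modes.
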(event `self.ReceiveBeginPlay`
  (`|ExecutionSequence`
    (:`then_0`
      (bind _asuhplayer_controller (cast `UHPlayerController` (`self.GetOwner`)))
      (set `self.PlayerController` _asuhplayer_controller))
    (:`then_1`
      (bind _returnvalue (`|CreateWidget` "/Game/UI/WBP_Crosshairs.WBP_Crosshairs_C"))
      (set `self.CrosshairsWidget` _returnvalue))))

(event `self.ReceiveTick`
  (params (DeltaSeconds :type "Float (single-precision)"))
  (bind _playercontroller (`self.PlayerController`))
  (bind _crosshairswidget (`self.CrosshairsWidget`))
  (bind _returnvalue (`UHPlayerController.GetControlMode` _playercontroller))
  (if (`KismetSystemLibrary.IsValid` _playercontroller)
    (if (`|EnumInequality` (`self.PreviousControlMode`) _returnvalue)
      (`|ExecutionSequence`
        (:`then_0`
          (switch `EControlMode` _returnvalue
            (:`Regular`
              (`Widget.RemoveFromParent` _crosshairswidget :!label _label))
            (:`UltraHandPicking`
              (`UserWidget.AddToPlayerScreen` _crosshairswidget 0))
            (:`UltraHandManipulation`
              (goto _label))
            (:`UltraHandTurning`
              (goto _label))))
        (:`then_1`
          (set `self.PreviousControlMode` _returnvalue))))))